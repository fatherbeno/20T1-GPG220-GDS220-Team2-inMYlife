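; Interactable VR door that a motion controller can grab and swing around its hinge.
; Grab stores the controller, turns off hinge physics and opens a gate so Tick yaws the hinge to face the controller's location.
; Drop by the same controller clears the reference, re-enables hinge physics and closes the gate.
; Both events print the controller reference's name for debugging.
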(event `self.ReceiveTick`
  (params (DeltaSeconds :type "Float (single-precision)"))
  (bind (_returnvalue_roll _returnvalue_pitch _returnvalue_yaw) (`KismetMathLibrary.BreakRotator` (`KismetMathLibrary.FindLookAtRotation` (`SceneComponent.K2_GetComponentLocation` (`self.Hinge`)) (`SceneComponent.K2_GetComponentLocation` (`self.ControllerReference`)))))
  (`/Engine/EditorBlueprintResources/StandardMacros.Gate` true :!label _label
    (:`Exit`
      (`SceneComponent.K2_SetWorldRotation` (`self.Hinge`) (`KismetMathLibrary.MakeRotator` 0.0 0.0 _returnvalue_yaw) false false))))

(event `/Game/BensTests/PlayerCharacterTest/NewVRController/BPI_PlayerInteraction.Grab`
  (params (MotionController :type "SceneComponent Object Reference"))
  (bind _output_get (set `self.ControllerReference` MotionController))
  (`KismetSystemLibrary.PrintString` (`KismetSystemLibrary.GetDisplayName` _output_get))
  (`PrimitiveComponent.SetSimulatePhysics` (`self.Hinge`) false)
  (goto _label :!via `Open`))

(event `/Game/BensTests/PlayerCharacterTest/NewVRController/BPI_PlayerInteraction.Drop`
  (params (MotionController :type "SceneComponent Object Reference"))
  (if (== MotionController (`self.ControllerReference`))
    (bind _output_get (set `self.ControllerReference` null))
    (`KismetSystemLibrary.PrintString` (`KismetSystemLibrary.GetDisplayName` _output_get))
    (`PrimitiveComponent.SetSimulatePhysics` (`self.Hinge`) true)
    (goto _label :!via `Close`)))

(fn `UserConstructionScript`
  (`parent.UserConstructionScript`))