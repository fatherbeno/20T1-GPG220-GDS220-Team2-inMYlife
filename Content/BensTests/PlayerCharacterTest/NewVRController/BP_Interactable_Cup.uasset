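; BP_Interactable_Cup is a test VR cup that a motion controller can grab and drop.
; Grab stores the controller, turns off physics on the cup mesh and attaches it to the controller in place.
; Drop restores physics and detaches, only for the holding controller.
; A Gate opened on grab and closed on drop filters Action from that controller, with nothing wired after it.
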(event `/Game/BensTests/PlayerCharacterTest/NewVRController/BPI_PlayerInteraction.Action`
  (params (MotionController :type "SceneComponent Object Reference"))
  ;[1 1 1] Grab NPC Boxes + if grabbed allow "Event Action"
  (if (== (`self.ControllerReference`) MotionController)
    (`/Engine/EditorBlueprintResources/StandardMacros.Gate` true :!label _label)))

(event `/Game/BensTests/PlayerCharacterTest/NewVRController/BPI_PlayerInteraction.Grab`
  (params (MotionController :type "SceneComponent Object Reference"))
  ;[1 1 1] Grab NPC Boxes + if grabbed allow "Event Action"
  (set `self.ControllerReference` MotionController)
  (`PrimitiveComponent.SetSimulatePhysics` (`self.CupMesh`) false)
  (`SceneComponent.K2_AttachToComponent` (`self.CupMesh`) (`self.ControllerReference`) "None" "KeepWorld" "KeepWorld" "KeepWorld" false)
  (goto _label :!via `Open`))

(event `/Game/BensTests/PlayerCharacterTest/NewVRController/BPI_PlayerInteraction.Drop`
  (params (MotionController :type "SceneComponent Object Reference"))
  ;[1 1 1] Grab NPC Boxes + if grabbed allow "Event Action"
  (if (== MotionController (`self.ControllerReference`))
    (set `self.ControllerReference` null)
    (`PrimitiveComponent.SetSimulatePhysics` (`self.CupMesh`) true)
    (`SceneComponent.K2_DetachFromComponent` (`self.CupMesh`) "KeepWorld" "KeepWorld" "KeepWorld" false)
    (goto _label :!via `Close`)))

(fn `UserConstructionScript`
  (`parent.UserConstructionScript`))