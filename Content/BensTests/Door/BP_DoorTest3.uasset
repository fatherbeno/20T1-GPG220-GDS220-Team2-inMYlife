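; Test VR door Blueprint whose hinge swings to follow whatever grabs it.
; PickupOLD turns off hinge physics and opens a gate, through which Tick sets the hinge's relative yaw from a world-space look-at toward the AttachTo target.
; The player MotionControllerPawn's drop event, bound on BeginPlay, restores hinge physics and closes the gate.
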(event `self.ReceiveTick`
  (params (DeltaSeconds :type "Float (single-precision)"))
  (`/Engine/EditorBlueprintResources/StandardMacros.Gate` true :!label _label
    (:`Exit`
      (bind (_returnvalue_roll _returnvalue_pitch _returnvalue_yaw) (`KismetMathLibrary.BreakRotator` (`KismetMathLibrary.FindLookAtRotation` (`SceneComponent.K2_GetComponentLocation` (`self.Hinge`)) (`SceneComponent.K2_GetComponentLocation` (stale `/Game/VirtualRealityBP/Blueprints/PickupActorInterface.PickupOLD` AttachTo)))))
      (`SceneComponent.K2_SetRelativeRotation` (`self.Hinge`) (`KismetMathLibrary.MakeRotator` 0.0 0.0 _returnvalue_yaw) false false))))

(event `/Game/VirtualRealityBP/Blueprints/PickupActorInterface.PickupOLD`
  (params (AttachTo :type "SceneComponent Object Reference"))
  (`PrimitiveComponent.SetSimulatePhysics` (`self.Hinge`) false)
  (goto _label :!via `Open`))

(event `self.ReceiveBeginPlay`
  (bind _asmotion_controller_pawn (cast `/Game/VirtualRealityBP/Blueprints/MotionControllerPawn` (`GameplayStatics.GetPlayerPawn` 0)))
  (add `/Game/VirtualRealityBP/Blueprints/MotionControllerPawn.DropEvent` _asmotion_controller_pawn (delegate `Drwhat`)))

(event `Drwhat`
  (`PrimitiveComponent.SetSimulatePhysics` (`self.Hinge`) true)
  (goto _label :!via `Close`))

(fn `UserConstructionScript`)