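; BP_Interactable_NPC is a VR dialogue-system test NPC that shows its configured name on a widget.
; BeginPlay fills the name widget from NPCInformation and caches the dialogue game mode and VR player.
; Tick rotates the name display toward the player's HMD camera after a short delay.
; Grab, Drop and Action events are empty; the attach, detach and gated StartDialogueSystem logic is disconnected, so it never runs.
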(event `self.ReceiveTick`
  (params (DeltaSeconds :type "Float (single-precision)"))
  (bind _playerreference (`self.PlayerReference`))
  ;[1 1 1] Rotate Widget to Always Face Player
  (`KismetSystemLibrary.Delay` 0.1)
  (`/Engine/EditorBlueprintResources/StandardMacros.IsValid` _playerreference
    (:`Is Valid`
      (`SceneComponent.K2_SetWorldRotation` (`self.NameDisplay`) (`KismetMathLibrary.FindLookAtRotation` (`self.K2_GetActorLocation` self) (`SceneComponent.K2_GetComponentLocation` (`/Game/BensTests/PlayerCharacterTest/NewVRController/MainVRCharacter.HMD_Camera` _playerreference))) false false))))

(event `self.ReceiveBeginPlay`
  (bind _npc_information_npc_name (break `/Game/BensTests/DialogueSystemTests/DialogueSystem/BPS_NPCDialogue_Test` (`self.NPC Information`)))
  ;[1 1 1] Initialise Widget/Cast to Apropriate Blueprints
  (set `self.NameOfNPC` _npc_information_npc_name)
  (bind _asbp_game_mode_dialogue_system (cast `/Game/BensTests/DialogueSystemTests/DialogueSystem/BP_GameMode_DialogueSystem` (`GameplayStatics.GetGameMode`)))
  (set `self.GamemodeReference` _asbp_game_mode_dialogue_system)
  (bind _aswbp_display_npcname (cast `/Game/BensTests/DialogueSystemTests/DialogueSystem/WBP_DisplayNPCName` (`WidgetComponent.GetUserWidgetObject` (`self.NameDisplay`))))
  (set `/Game/BensTests/DialogueSystemTests/DialogueSystem/WBP_DisplayNPCName.DisplayedName` (`KismetTextLibrary.Conv_NameToText` (`self.NameOfNPC`)) _aswbp_display_npcname)
  (bind _asmain_vrcharacter (cast `/Game/BensTests/PlayerCharacterTest/NewVRController/MainVRCharacter` (`GameplayStatics.GetPlayerCharacter` 0)))
  (set `self.PlayerReference` _asmain_vrcharacter))

(event `/Game/BensTests/PlayerCharacterTest/NewVRController/BPI_PlayerInteraction.Action`
  (params (MotionController :type "SceneComponent Object Reference"))
  ;[1 1 1] Grab NPC Boxes + if grabbed allow "Event Action"
)

(event `/Game/BensTests/PlayerCharacterTest/NewVRController/BPI_PlayerInteraction.Grab`
  (params (MotionController :type "SceneComponent Object Reference"))
  ;[1 1 1] Grab NPC Boxes + if grabbed allow "Event Action"
)

(event `/Game/BensTests/PlayerCharacterTest/NewVRController/BPI_PlayerInteraction.Drop`
  (params (MotionController :type "SceneComponent Object Reference"))
  ;[1 1 1] Grab NPC Boxes + if grabbed allow "Event Action"
)

(fn `UserConstructionScript`
  (`parent.UserConstructionScript`))