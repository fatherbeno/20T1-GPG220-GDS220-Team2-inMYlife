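; AI controller for dialogue NPCs that walks the pawn to or away from set locations.
; On BeginPlay it caches the controlled pawn as a BP_Character_DialogueNPC.
; The walk-to event moves to WalkToLocation, then focuses on the player on success.
; The walk-away event waits briefly, clears focus, moves to WalkAwayLocation, then refocuses on the player after another short delay.
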(event `self.ReceiveBeginPlay`
  (bind _asbp_character_dialogue_npc (cast `/Game/BensTests/DialogueSystemTests/DialogueSystem/AI/BP_Character_DialogueNPC` (`self.K2_GetPawn`)))
  (set `self.PawnReference` _asbp_character_dialogue_npc))

(event `EventWalkToLocation`
  (`|AIMoveTo` (`self.PawnReference`) (`self.WalkToLocation`) null
    (:`OnSuccess`
      (`self.K2_SetFocus` (`GameplayStatics.GetPlayerCharacter` 0)))))

(event `EventWalkAwayLocation`
  (`KismetSystemLibrary.Delay` 1.0)
  (`self.K2_ClearFocus`)
  (`|AIMoveTo` (`self.PawnReference`) (`self.WalkAwayLocation`) null
    (:`OnSuccess`
      (`KismetSystemLibrary.Delay` 1.0)
      (`self.K2_SetFocus` (`GameplayStatics.GetPlayerCharacter` 0)))))

(fn `UserConstructionScript`)