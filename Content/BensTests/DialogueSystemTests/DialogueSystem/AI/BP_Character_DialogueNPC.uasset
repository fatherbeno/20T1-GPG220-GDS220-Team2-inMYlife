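; Dialogue-system NPC character for a VR game, with a floating name display and walk-to and walk-away destinations.
; On BeginPlay it fills the name widget from its NPC info, caches the game mode and VR player, and passes both destinations to its dialogue AI controller.
; Tick, throttled by a 0.1-second Delay, rotates the name display toward the player's HMD camera, using the actor's location as origin.
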(event `self.ReceiveTick`
  (params (DeltaSeconds :type "Float (single-precision)"))
  (bind _playerreference (`self.PlayerReference`))
  ;[1 1 1] Rotate Widget to Always Face Player
  (`KismetSystemLibrary.Delay` 0.1)
  (`/Engine/EditorBlueprintResources/StandardMacros.IsValid` _playerreference
    (:`Is Valid`
      (`SceneComponent.K2_SetWorldRotation` (`self.NameDisplay`) (`KismetMathLibrary.FindLookAtRotation` (`self.K2_GetActorLocation` self) (`SceneComponent.K2_GetComponentLocation` (`/Game/BensTests/PlayerCharacterTest/NewVRController/MainVRCharacter.HMD_Camera` _playerreference))) false false))))

(event `self.ReceiveBeginPlay`
  (bind _npc_information_npc_name (break `/Game/BensTests/DialogueSystemTests/DialogueSystem/BPS_NPCDialogue_Test` (`self.NPC Information`)))
  ;[1 1 1] Initialise Widget/Cast to Apropriate Blueprints
  (set `self.NameOfNPC` _npc_information_npc_name)
  (bind _asbp_game_mode_dialogue_system (cast `/Game/BensTests/DialogueSystemTests/DialogueSystem/BP_GameMode_DialogueSystem` (`GameplayStatics.GetGameMode`)))
  (set `self.GamemodeReference` _asbp_game_mode_dialogue_system)
  (bind _aswbp_display_npcname (cast `/Game/BensTests/DialogueSystemTests/DialogueSystem/WBP_DisplayNPCName` (`WidgetComponent.GetUserWidgetObject` (`self.NameDisplay`))))
  (set `/Game/BensTests/DialogueSystemTests/DialogueSystem/WBP_DisplayNPCName.DisplayedName` (`KismetTextLibrary.Conv_NameToText` (`self.NameOfNPC`)) _aswbp_display_npcname)
  (bind _asmain_vrcharacter (cast `/Game/BensTests/PlayerCharacterTest/NewVRController/MainVRCharacter` (`GameplayStatics.GetPlayerCharacter` 0)))
  (set `self.PlayerReference` _asmain_vrcharacter)
  (bind _asbp_ai_controller_dialogue_npc (cast `/Game/BensTests/DialogueSystemTests/DialogueSystem/AI/BP_AiController_DialogueNPC` (`self.GetController`)))
  (set `/Game/BensTests/DialogueSystemTests/DialogueSystem/AI/BP_AiController_DialogueNPC.WalkToLocation` (`self.WalkToLocation`) _asbp_ai_controller_dialogue_npc)
  (set `/Game/BensTests/DialogueSystemTests/DialogueSystem/AI/BP_AiController_DialogueNPC.WalkAwayLocation` (`self.WalkAwayLocation`) _asbp_ai_controller_dialogue_npc))

(fn `UserConstructionScript`)