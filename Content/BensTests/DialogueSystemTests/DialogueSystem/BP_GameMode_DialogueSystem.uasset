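; Test game mode that runs a VR dialogue system for interactable NPCs.
; StartDialogueSystem finds the NPC by name, copies its dialogue and choice arrays, then spawns a dialogue widget actor attached in front of the HMD camera.
; Widget-called events step through lines, spawn choice boxes on matching line indices and hold progression until a choice executes.
; Laser pointers and the menu-active flag are set during dialogue and cleared when it ends.
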(event `StartDialogueSystem`
  (params (NameOfNPC :type Name))
  ;[1 1 1] Extract Data from Specific NPC
  (bind _outactors (`GameplayStatics.GetAllActorsOfClass` "/Game/BensTests/DialogueSystemTests/DialogueSystem/BP_Interactable_NPC.BP_Interactable_NPC_C"))
  (for _array_element _outactors
    (bind (_npc_information_npc_name _npc_information_npc_dialogue _npc_information_playerchoices) (break `/Game/BensTests/DialogueSystemTests/DialogueSystem/BPS_NPCDialogue_Test` (`/Game/BensTests/DialogueSystemTests/DialogueSystem/BP_Interactable_NPC.NPC Information` _array_element)))
    (if (== NameOfNPC _npc_information_npc_name)
      (`|ExecutionSequence`
        (:`then_0`
          (set `self.dialogueArray` _npc_information_npc_dialogue)
          (set `self.choiceTextArray` _npc_information_playerchoices)
          ;[0 1 0.002357] Display Dialogue Box
          (`self.resetLoop`)
          (`self.DisplayDialogueSystem`)
          (`self.Setup Display Choice Boxes`))
        (:`then_1`
          (goto _label :!via `Close`)))))
  (`|ExecutionSequence`
    (:`then_0`
      (`/Engine/EditorBlueprintResources/StandardMacros.Gate` false :!label _label
        (:`Exit`
          (for _ (range 10)
            (`KismetSystemLibrary.PrintString` (`KismetStringLibrary.Concat_StrStr` "                                 THE NAME \"" (`KismetStringLibrary.Conv_NameToString` NameOfNPC) "\" IS NOT A NPC IN THE DIALOGUE SYSTEM") true false (struct :`G` 0.66 :`B` 1.0 :`A` 1.0) 5.0)))))
    (:`then_1`
      (goto _label :!via `Open`))))

(event `self.ReceiveBeginPlay`
  ;[1 1 1] Initialise Dialogue System
  (bind _asmain_vrcharacter (cast `/Game/BensTests/PlayerCharacterTest/NewVRController/MainVRCharacter` (`GameplayStatics.GetPlayerCharacter` 0)))
  (set `self.PlayerReference` _asmain_vrcharacter))

(event `resetLoop`
  ;[0 0.9797 1] Reset Initial "Loop" Values
  (set `self.lastIndex` (`KismetArrayLibrary.Array_LastIndex` (`self.dialogueArray`)))
  (set `self.firstIndex` 0)
  (set `self.arrayIndex` 0)
  (set `self.currentChoiceNumber` 0)
  (set `self.currentDialogue` (`|GetArrayItem` (`self.dialogueArray`))))

(event `dialogueBoxExecute`
  (bind _arrayindex (`self.arrayIndex`))
  (bind _playerreference (`self.PlayerReference`))
  ;[1 1 1] Recieve Inputs from Widgets
  (if (not (`self.currentChoiceTrigger`))
    ;[1 1 1] Cycle Through Dialogue
    (set `self.currentChoiceTrigger` false :!label _label_2)
    (if (< _arrayindex (`self.lastIndex`))
      (set `self.arrayIndex` (+ _arrayindex 1))
      (set `self.currentDialogue` (`|GetArrayItem` (`self.dialogueArray`) (`self.arrayIndex`)))
      (`self.Setup Display Choice Boxes`)
      (else
        ;[1 0 0.8275] Once Dialogue Finishes, Destroy Dialogue Box
        (`self.K2_DestroyActor` (`self.NPCDialogue_WidgetActorReference`))
        (set `self.NPCDialogue_WidgetActorReference` null)
        ;[1 1 1] Disable Laser Pointers + Enable Player Actions
        (set `WidgetInteractionComponent.bShowDebug` false (`/Game/BensTests/PlayerCharacterTest/NewVRController/MainVRCharacter.L_WidgetInteraction` _playerreference))
        (set `WidgetInteractionComponent.bShowDebug` false (`/Game/BensTests/PlayerCharacterTest/NewVRController/MainVRCharacter.R_WidgetInteraction` _playerreference))
        (set `/Game/BensTests/PlayerCharacterTest/NewVRController/MainVRCharacter.IsMenuActive` false _playerreference)))))

(event `dialogueChoiceExecute`
  ;[1 1 1] Recieve Inputs from Widgets
  (if (`self.currentChoiceTrigger`)
    ;;[1 0 0.8275] Destroy Choice Boxes
    (`self.K2_DestroyActor` (`self.PlayerDialogue_WidgetActorReference`))
    (set `self.PlayerDialogue_WidgetActorReference` null)
    (goto _label_2)))

(event `Setup Display Choice Boxes`
  ;[0.1791 1 0] Setup then Display Choice Boxes
  (for _array_element (`self.choiceTextArray`)
    (if (== (`self.arrayIndex`) (break `/Game/BensTests/DialogueSystemTests/DialogueSystem/BPS_PlayerChoices_Test` _array_element))
      (`|ExecutionSequence`
        (:`then_0`
          (set `self.choiceOneText` (`.Choice1_9_B08A71C84FBF078C422AF688CB77A21B` (break `/Game/BensTests/DialogueSystemTests/DialogueSystem/BPS_PlayerChoices_Test` _array_element))))
        (:`then_1`
          (set `self.choiceTwoText` (`.Choice2_10_406CEC6C404711FD8910DEB7486E739E` (break `/Game/BensTests/DialogueSystemTests/DialogueSystem/BPS_PlayerChoices_Test` _array_element))))
        (:`then_2`
          (set `self.choiceThreeText` (`.Choice3_11_414B552C4B3070EF09307CB483A18EC6` (break `/Game/BensTests/DialogueSystemTests/DialogueSystem/BPS_PlayerChoices_Test` _array_element))))
        (:`then_3`
          (set `self.choiceFourText` (`.Choice4_12_7BFCD47A4CC5969A024ED99709DA51A6` (break `/Game/BensTests/DialogueSystemTests/DialogueSystem/BPS_PlayerChoices_Test` _array_element)))
          (set `self.currentChoiceTrigger` true)
          (`self.DisplayChoiceSystem`))))))

(fn `DisplayChoiceSystem`
  (locals (ForwardMenuDistance :type "Float (double-precision)" :default 150.0) (UpwardsMenuDistance :type "Float (double-precision)" :default -30.0))
  (bind _playerdialogue_widgetactorreference (`self.PlayerDialogue_WidgetActorReference`))
  (bind _hmd_camera (`/Game/BensTests/PlayerCharacterTest/NewVRController/MainVRCharacter.HMD_Camera` (`self.PlayerReference`)))
  (bind _returnvalue_roll (`KismetMathLibrary.BreakRotator` (`SceneComponent.K2_GetComponentRotation` (`/Game/BensTests/PlayerCharacterTest/NewVRController/MainVRCharacter.HMD_Camera` (`self.PlayerReference`)))))
  (bind (_returnvalue_roll_2 _returnvalue_pitch _returnvalue_yaw) (`KismetMathLibrary.BreakRotator` (`SceneComponent.K2_GetComponentRotation` _hmd_camera)))
  (bind (_returnvalue_roll_3 _returnvalue_pitch_2 _returnvalue_yaw_2) (`KismetMathLibrary.BreakRotator` (`KismetMathLibrary.FindLookAtRotation` (`self.K2_GetActorLocation` (`self.PlayerDialogue_WidgetActorReference`)) (`SceneComponent.K2_GetComponentLocation` (`/Game/BensTests/PlayerCharacterTest/NewVRController/MainVRCharacter.HMD_Camera` (`self.PlayerReference`))))))
  (bind _returnvalue (`KismetMathLibrary.MakeRotator` 0.0 _returnvalue_pitch _returnvalue_yaw))
  ;[1 1 1] Spawn Widget Actor
  (bind _returnvalue_2 (`|SpawnActorFromClass` (`self.PlayerDialogue_WidgetClassReference`) (`KismetMathLibrary.MakeTransform` (0.0 0.0 0.0) (struct) (0.1 0.1 0.1)) "Undefined" "OverrideRootScale" null null))
  (bind _asbp_player_dialogue_options_actor_test (cast `/Game/BensTests/DialogueSystemTests/DialogueSystem/BP_PlayerDialogueOptionsActor_Test` _returnvalue_2))
  (set `self.PlayerDialogue_WidgetActorReference` _asbp_player_dialogue_options_actor_test)
  ;[1 1 1] Rotate/Translate Widget Actor
  (`self.K2_SetActorLocation` (`self.PlayerDialogue_WidgetActorReference`) (+ (`SceneComponent.K2_GetComponentLocation` _hmd_camera) (+ (* (`KismetMathLibrary.GetForwardVector` _returnvalue) (`local.ForwardMenuDistance`)) (* (`KismetMathLibrary.GetUpVector` _returnvalue) (`local.UpwardsMenuDistance`)))) false false)
  (`self.K2_SetActorRotation` (`self.PlayerDialogue_WidgetActorReference`) (`KismetMathLibrary.MakeRotator` (* _returnvalue_roll -1.0) _returnvalue_pitch_2 _returnvalue_yaw_2) false)
  ;[1 1 1] Attach Widget to Camera
  (`SceneComponent.SetVisibility` (`/Game/BensTests/DialogueSystemTests/DialogueSystem/BP_PlayerDialogueOptionsActor_Test.PlayerDialogueOptions` _playerdialogue_widgetactorreference) true false)
  (`self.K2_AttachToComponent` _playerdialogue_widgetactorreference (`/Game/BensTests/PlayerCharacterTest/NewVRController/MainVRCharacter.HMD_Camera` (`self.PlayerReference`)) "None" "KeepWorld" "KeepWorld" "KeepWorld" false))

(fn `DisplayDialogueSystem`
  (locals (ForwardMenuDistance :type "Float (double-precision)" :default 150.0) (UpwardsMenuDistance :type "Float (double-precision)" :default 30.0))
  (bind _npcdialogue_widgetactorreference (`self.NPCDialogue_WidgetActorReference`))
  (bind _playerreference (`self.PlayerReference`))
  (bind _hmd_camera (`/Game/BensTests/PlayerCharacterTest/NewVRController/MainVRCharacter.HMD_Camera` (`self.PlayerReference`)))
  (bind _returnvalue_roll (`KismetMathLibrary.BreakRotator` (`SceneComponent.K2_GetComponentRotation` (`/Game/BensTests/PlayerCharacterTest/NewVRController/MainVRCharacter.HMD_Camera` (`self.PlayerReference`)))))
  (bind (_returnvalue_roll_2 _returnvalue_pitch _returnvalue_yaw) (`KismetMathLibrary.BreakRotator` (`SceneComponent.K2_GetComponentRotation` _hmd_camera)))
  (bind (_returnvalue_roll_3 _returnvalue_pitch_2 _returnvalue_yaw_2) (`KismetMathLibrary.BreakRotator` (`KismetMathLibrary.FindLookAtRotation` (`self.K2_GetActorLocation` (`self.NPCDialogue_WidgetActorReference`)) (`SceneComponent.K2_GetComponentLocation` (`/Game/BensTests/PlayerCharacterTest/NewVRController/MainVRCharacter.HMD_Camera` (`self.PlayerReference`))))))
  (bind _returnvalue (`KismetMathLibrary.MakeRotator` 0.0 _returnvalue_pitch _returnvalue_yaw))
  ;[1 1 1] Spawn Widget Actor
  (bind _returnvalue_2 (`|SpawnActorFromClass` (`self.NPCDialogue_WidgetClassReference`) (`KismetMathLibrary.MakeTransform` (0.0 0.0 0.0) (struct) (0.1 0.1 0.1)) "Undefined" "OverrideRootScale" null null))
  (bind _asbp_npcdialogue_actor_test (cast `/Game/BensTests/DialogueSystemTests/DialogueSystem/BP_NPCDialogueActor_Test` _returnvalue_2))
  (set `self.NPCDialogue_WidgetActorReference` _asbp_npcdialogue_actor_test)
  ;[1 1 1] Rotate/Translate Widget Actor
  (`self.K2_SetActorLocation` (`self.NPCDialogue_WidgetActorReference`) (+ (`SceneComponent.K2_GetComponentLocation` _hmd_camera) (+ (* (`KismetMathLibrary.GetForwardVector` _returnvalue) (`local.ForwardMenuDistance`)) (* (`KismetMathLibrary.GetUpVector` _returnvalue) (`local.UpwardsMenuDistance`)))) false false)
  (`self.K2_SetActorRotation` (`self.NPCDialogue_WidgetActorReference`) (`KismetMathLibrary.MakeRotator` (* _returnvalue_roll -1.0) _returnvalue_pitch_2 _returnvalue_yaw_2) false)
  ;[1 1 1] Attach Widget to Camera
  (`SceneComponent.SetVisibility` (`/Game/BensTests/DialogueSystemTests/DialogueSystem/BP_NPCDialogueActor_Test.NPCDialogue` _npcdialogue_widgetactorreference) true false)
  (`self.K2_AttachToComponent` _npcdialogue_widgetactorreference (`/Game/BensTests/PlayerCharacterTest/NewVRController/MainVRCharacter.HMD_Camera` (`self.PlayerReference`)) "None" "KeepWorld" "KeepWorld" "KeepWorld" false)
  ;[1 1 1] Show Laser Pointers for Player
  (set `WidgetInteractionComponent.bShowDebug` true (`/Game/BensTests/PlayerCharacterTest/NewVRController/MainVRCharacter.L_WidgetInteraction` _playerreference))
  (set `WidgetInteractionComponent.bShowDebug` true (`/Game/BensTests/PlayerCharacterTest/NewVRController/MainVRCharacter.R_WidgetInteraction` _playerreference))
  (set `/Game/BensTests/PlayerCharacterTest/NewVRController/MainVRCharacter.IsMenuActive` true _playerreference))

(fn `UserConstructionScript`)