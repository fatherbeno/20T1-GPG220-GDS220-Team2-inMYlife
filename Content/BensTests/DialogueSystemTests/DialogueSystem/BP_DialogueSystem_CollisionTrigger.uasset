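; A one-shot collision trigger that starts a dialogue with a named NPC in the dialogue system.
; On the first overlap with any actor, it finds the dialogue NPC matching NameOfNPC and passes its AI controller to the dialogue GameMode.
; It then fires the controller's walk-to-location event, starts the dialogue through the GameMode and destroys itself after a short delay.
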(event `self.ReceiveBeginPlay`
  ;[1 1 1] Get Gamemode Reference
  (bind _asbp_game_mode_dialogue_system (cast `/Game/BensTests/DialogueSystemTests/DialogueSystem/BP_GameMode_DialogueSystem` (`GameplayStatics.GetGameMode`)))
  (set `self.GamemodeReference` _asbp_game_mode_dialogue_system))

(event `self.CollisionBox.OnComponentBeginOverlap`
  (params (OverlappedComponent :type "PrimitiveComponent Object Reference") (OtherActor :type "Actor Object Reference") (OtherComp :type "PrimitiveComponent Object Reference") (OtherBodyIndex :type Integer) (bFromSweep :type Boolean) (SweepResult :type "HitResult Structure (by ref)"))
  (`/Engine/EditorBlueprintResources/StandardMacros.DoOnce` false
    (:`Completed`
      (bind _outactors (`GameplayStatics.GetAllActorsOfClass` "/Game/BensTests/DialogueSystemTests/DialogueSystem/AI/BP_Character_DialogueNPC.BP_Character_DialogueNPC_C"))
      (for _array_element _outactors
        (bind _npc_information_npc_name (break `/Game/BensTests/DialogueSystemTests/DialogueSystem/BPS_NPCDialogue_Test` (`/Game/BensTests/DialogueSystemTests/DialogueSystem/AI/BP_Character_DialogueNPC.NPC Information` _array_element)))
        (if (== (`self.NameOfNPC`) _npc_information_npc_name)
          (bind _output_get (set `self.NonPlayerCharacterReference` _array_element))
          (bind _asbp_ai_controller_dialogue_npc (cast `/Game/BensTests/DialogueSystemTests/DialogueSystem/AI/BP_AiController_DialogueNPC` (`Pawn.GetController` _output_get)))
          (bind _output_get_2 (set `/Game/BensTests/DialogueSystemTests/DialogueSystem/BP_GameMode_DialogueSystem.CurrentAiControllerReference` _asbp_ai_controller_dialogue_npc (`self.GamemodeReference`)))
          (`|ExecutionSequence`
            (:`then_0`
              (`/Game/BensTests/DialogueSystemTests/DialogueSystem/AI/BP_AiController_DialogueNPC.EventWalkToLocation` _output_get_2))
            (:`then_1`
              ;[1 1 1] Start Dialogue System
              (`/Game/BensTests/DialogueSystemTests/DialogueSystem/BP_GameMode_DialogueSystem.StartDialogueSystem` (`self.GamemodeReference`) (`self.NameOfNPC`))
              (`KismetSystemLibrary.Delay` 0.2)
              (`self.K2_DestroyActor`))))))))

(fn `UserConstructionScript`)