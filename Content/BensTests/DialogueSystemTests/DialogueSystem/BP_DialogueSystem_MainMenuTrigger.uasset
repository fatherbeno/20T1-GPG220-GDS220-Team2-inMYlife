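; A one-shot trigger volume that starts dialogue in the dialogue system, named for use in the main menu.
; On overlap it picks one of two NPC names from the save's HasPlayedBefore flag and finds the matching BP_Character_DialogueNPC.
; It hands that NPC's AI controller to the dialogue game mode, starts the matching dialogue, then destroys itself.
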(event `self.ReceiveBeginPlay`
  (bind _asbp_game_mode_dialogue_system (cast `/Game/BensTests/DialogueSystemTests/DialogueSystem/BP_GameMode_DialogueSystem` (`GameplayStatics.GetGameMode`)))
  (set `self.GamemodeReference` _asbp_game_mode_dialogue_system))

(event `self.Box.OnComponentBeginOverlap`
  (params (OverlappedComponent :type "PrimitiveComponent Object Reference") (OtherActor :type "Actor Object Reference") (OtherComp :type "PrimitiveComponent Object Reference") (OtherBodyIndex :type Integer) (bFromSweep :type Boolean) (SweepResult :type "HitResult Structure (by ref)"))
  (`/Engine/EditorBlueprintResources/StandardMacros.DoOnce` false
    (:`Completed`
      (`|ExecutionSequence`
        (:`then_0`
          (if (`/Game/BensTests/DataSerialisation/BP_SaveGame.HasPlayedBefore` (`/Game/BensTests/DialogueSystemTests/DialogueSystem/BP_GameMode_DialogueSystem.SaveGameData` (`self.GamemodeReference`)))
            (set `self.NameOfNPC` (`self.PlayedBefore`))
            (else
              (set `self.NameOfNPC` (`self.NotPlayedBefore`)))))
        (:`then_1`
          (bind _outactors (`GameplayStatics.GetAllActorsOfClass` "/Game/BensTests/DialogueSystemTests/DialogueSystem/AI/BP_Character_DialogueNPC.BP_Character_DialogueNPC_C"))
          (for _array_element _outactors
            (bind _npc_information_npc_name (break `/Game/BensTests/DialogueSystemTests/DialogueSystem/BPS_NPCDialogue_Test` (`/Game/BensTests/DialogueSystemTests/DialogueSystem/AI/BP_Character_DialogueNPC.NPC Information` _array_element)))
            (if (== (`self.NameOfNPC`) _npc_information_npc_name)
              (bind _output_get (set `self.NonPlayerCharacterReference` _array_element))
              (bind _asbp_ai_controller_dialogue_npc (cast `/Game/BensTests/DialogueSystemTests/DialogueSystem/AI/BP_AiController_DialogueNPC` (`Pawn.GetController` _output_get)))
              (set `/Game/BensTests/DialogueSystemTests/DialogueSystem/BP_GameMode_DialogueSystem.CurrentAiControllerReference` _asbp_ai_controller_dialogue_npc (`self.GamemodeReference`)))))
        (:`then_2`
          (if (`/Game/BensTests/DataSerialisation/BP_SaveGame.HasPlayedBefore` (`/Game/BensTests/DialogueSystemTests/DialogueSystem/BP_GameMode_DialogueSystem.SaveGameData` (`self.GamemodeReference`)))
            (`/Game/BensTests/DialogueSystemTests/DialogueSystem/BP_GameMode_DialogueSystem.StartDialogueSystem` (`self.GamemodeReference`) (`self.PlayedBefore`))
            (else
              (`/Game/BensTests/DialogueSystemTests/DialogueSystem/BP_GameMode_DialogueSystem.StartDialogueSystem` (`self.GamemodeReference`) (`self.NotPlayedBefore`))))
          (`self.K2_DestroyActor`))))))

(fn `UserConstructionScript`)