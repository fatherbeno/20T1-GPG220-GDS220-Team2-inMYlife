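; Test VR dialogue system that shows NPC lines and four-option player choices on widget actors attached to the HMD camera.
; Dialogue-box and choice events step through parallel dialogue and trigger arrays, spawning choices when flagged.
; Widget-interaction debug lasers and a menu flag are set while dialogue shows, then cleared when it ends.
; Player binding, NPC name lookup, loop reset and initial display are unwired, so triggering only clears existing widgets.
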(event `self.ReceiveBeginPlay`
  ;[1 1 1] Initialise Dialogue System
)

(event `TriggerNPCTalkingInteraction_Event` :!signature `self.TriggerNPCTalkingInteraction`
  (params (NameOfNPC :type Name))
  (bind _npcdialogue_widgetactorreference (`self.NPCDialogue_WidgetActorReference`))
  (bind _playerdialogueoptions_widgetactorreference (`self.PlayerDialogueOptions_WidgetActorReference`))
  ;[1 1 1] Initialise Dialogue System
  (set `self.whichNPC` NameOfNPC)
  (`|ExecutionSequence`
    (:`then_0`
      (`/Engine/EditorBlueprintResources/StandardMacros.IsValid` _playerdialogueoptions_widgetactorreference
        (:`Is Valid`
          (`self.K2_DestroyActor` _playerdialogueoptions_widgetactorreference)
          (set `self.PlayerDialogueOptions_WidgetActorReference` null))))
    (:`then_1`
      (`/Engine/EditorBlueprintResources/StandardMacros.IsValid` _npcdialogue_widgetactorreference
        (:`Is Valid`
          (`self.K2_DestroyActor` _npcdialogue_widgetactorreference)
          (set `self.NPCDialogue_WidgetActorReference` null))))
    (:`then_2`
      ;[1 1 1] Extract Data from Specific NPC
      (for _array_element (`self.listOfNPCs`)
        _))))

(event `resetLoop`
  ;[0 0.9797 1] Reset Initial "Loop" Values
)

(event `dialogueBoxExecute`
  (bind _arrayindex (`self.arrayIndex`))
  (bind _playerreference (`self.PlayerReference`))
  ;[1 1 1] Recieve Inputs from Widgets
  (if (not (`self.currentChoiceTrigger`))
    ;[1 1 1] Cycle Through Dialogue
    (if (< _arrayindex (`self.lastIndex`)) :!label _label
      (bind _output_get (set `self.arrayIndex` (+ _arrayindex 1)))
      (set `self.currentChoiceTrigger` (`|GetArrayItem` (`self.choiceTriggerArray`) _output_get))
      (set `self.currentDialogue` (`|GetArrayItem` (`self.dialogueArray`) (`self.arrayIndex`)))
      (`self.Setup Display Choice Boxes`)
      (else
        ;[1 0 0.8275] Once Dialogue Finishes, Destroy Dialogue Box
        (`self.K2_DestroyActor` (`self.NPCDialogue_WidgetActorReference`))
        (set `self.NPCDialogue_WidgetActorReference` null)
        ;[1 1 1] Disable Laser Pointers + Enable Player Actions
        (set `WidgetInteractionComponent.bShowDebug` false (`/Game/BensTests/PlayerCharacterTest/NewVRController/MainVRCharacter.L_WidgetInteraction` _playerreference))
        (set `WidgetInteractionComponent.bShowDebug` false (`/Game/BensTests/PlayerCharacterTest/NewVRController/MainVRCharacter.R_WidgetInteraction` _playerreference))
        (set `/Game/BensTests/PlayerCharacterTest/NewVRController/MainVRCharacter.IsMenuActive` false _playerreference)))))

(event `dialogueChoiceExecute`
  ;[1 1 1] Recieve Inputs from Widgets
  (if (`self.currentChoiceTrigger`)
    ;;[1 0 0.8275] Destroy Choice Boxes
    (`self.K2_DestroyActor` (`self.PlayerDialogueOptions_WidgetActorReference`))
    (set `self.PlayerDialogueOptions_WidgetActorReference` null)
    (goto _label)))

(event `Setup Display Choice Boxes`
  (bind (_output_whichdialogue _output_choice1 _output_choice2 _output_choice3 _output_choice4) (break `/Game/BensTests/DialogueSystemTests/DialogueSystem/BPS_PlayerChoices_Test` (`|GetArrayItem` (`self.choiceTextArray`) (`self.currentChoiceNumber`))))
  ;[0.1791 1 0] Setup then Display Choice Boxes
  (if (`self.currentChoiceTrigger`)
    (`|ExecutionSequence`
      (:`then_0`
        (set `self.choiceOneText` _output_choice1))
      (:`then_1`
        (set `self.choiceTwoText` _output_choice2))
      (:`then_2`
        (set `self.choiceThreeText` _output_choice3))
      (:`then_3`
        (set `self.choiceFourText` _output_choice4)
        (set `self.currentChoiceNumber` (+ (`self.currentChoiceNumber`) 1))
        (`self.DisplayChoiceSystem`)))))

(fn `DisplayChoiceSystem`
  (locals (ForwardMenuDistance :type "Float (double-precision)" :default 150.0) (UpwardsMenuDistance :type "Float (double-precision)" :default -30.0))
  (bind _playerdialogueoptions_widgetactorreference (`self.PlayerDialogueOptions_WidgetActorReference`))
  (bind _hmd_camera (`/Game/BensTests/PlayerCharacterTest/NewVRController/MainVRCharacter.HMD_Camera` (`self.PlayerReference`)))
  (bind _returnvalue_roll (`KismetMathLibrary.BreakRotator` (`SceneComponent.K2_GetComponentRotation` (`/Game/BensTests/PlayerCharacterTest/NewVRController/MainVRCharacter.HMD_Camera` (`self.PlayerReference`)))))
  (bind (_returnvalue_roll_2 _returnvalue_pitch _returnvalue_yaw) (`KismetMathLibrary.BreakRotator` (`SceneComponent.K2_GetComponentRotation` _hmd_camera)))
  (bind (_returnvalue_roll_3 _returnvalue_pitch_2 _returnvalue_yaw_2) (`KismetMathLibrary.BreakRotator` (`KismetMathLibrary.FindLookAtRotation` (`self.K2_GetActorLocation` (`self.PlayerDialogueOptions_WidgetActorReference`)) (`SceneComponent.K2_GetComponentLocation` (`/Game/BensTests/PlayerCharacterTest/NewVRController/MainVRCharacter.HMD_Camera` (`self.PlayerReference`))))))
  (bind _returnvalue (`KismetMathLibrary.MakeRotator` 0.0 _returnvalue_pitch _returnvalue_yaw))
  ;[1 1 1] Spawn Widget Actor
  (bind _returnvalue_2 (`|SpawnActorFromClass` (`self.PlayerDialogueOptions_WidgetClassReference`) (`KismetMathLibrary.MakeTransform` (0.0 0.0 0.0) (struct) (0.1 0.1 0.1)) "Undefined" "OverrideRootScale" null null))
  (bind _asbp_player_dialogue_options_actor_test (cast `/Game/BensTests/DialogueSystemTests/DialogueSystem/BP_PlayerDialogueOptionsActor_Test` _returnvalue_2))
  (set `self.PlayerDialogueOptions_WidgetActorReference` _asbp_player_dialogue_options_actor_test)
  ;[1 1 1] Rotate/Translate Widget Actor
  (`self.K2_SetActorLocation` (`self.PlayerDialogueOptions_WidgetActorReference`) (+ (`SceneComponent.K2_GetComponentLocation` _hmd_camera) (+ (* (`KismetMathLibrary.GetForwardVector` _returnvalue) (`local.ForwardMenuDistance`)) (* (`KismetMathLibrary.GetUpVector` _returnvalue) (`local.UpwardsMenuDistance`)))) false false)
  (`self.K2_SetActorRotation` (`self.PlayerDialogueOptions_WidgetActorReference`) (`KismetMathLibrary.MakeRotator` (* _returnvalue_roll -1.0) _returnvalue_pitch_2 _returnvalue_yaw_2) false)
  ;[1 1 1] Attach Widget to Camera
  (`SceneComponent.SetVisibility` (`/Game/BensTests/DialogueSystemTests/DialogueSystem/BP_PlayerDialogueOptionsActor_Test.PlayerDialogueOptions` _playerdialogueoptions_widgetactorreference) true false)
  (`self.K2_AttachToComponent` _playerdialogueoptions_widgetactorreference (`/Game/BensTests/PlayerCharacterTest/NewVRController/MainVRCharacter.HMD_Camera` (`self.PlayerReference`)) "None" "KeepWorld" "KeepWorld" "KeepWorld" false))

(fn `DisplayDialogueSystem`
  (locals (ForwardMenuDistance :type "Float (double-precision)" :default 150.0) (UpwardsMenuDistance :type "Float (double-precision)" :default 30.0))
  (bind _npcdialogue_widgetactorreference (`self.NPCDialogue_WidgetActorReference`))
  (bind _playerreference (`self.PlayerReference`))
  (bind _hmd_camera (`/Game/BensTests/PlayerCharacterTest/NewVRController/MainVRCharacter.HMD_Camera` (`self.PlayerReference`)))
  (bind _returnvalue_roll (`KismetMathLibrary.BreakRotator` (`SceneComponent.K2_GetComponentRotation` (`/Game/BensTests/PlayerCharacterTest/NewVRController/MainVRCharacter.HMD_Camera` (`self.PlayerReference`)))))
  (bind (_returnvalue_roll_2 _returnvalue_pitch _returnvalue_yaw) (`KismetMathLibrary.BreakRotator` (`SceneComponent.K2_GetComponentRotation` _hmd_camera)))
  (bind (_returnvalue_roll_3 _returnvalue_pitch_2 _returnvalue_yaw_2) (`KismetMathLibrary.BreakRotator` (`KismetMathLibrary.FindLookAtRotation` (`self.K2_GetActorLocation` (`self.NPCDialogue_WidgetActorReference`)) (`SceneComponent.K2_GetComponentLocation` (`/Game/BensTests/PlayerCharacterTest/NewVRController/MainVRCharacter.HMD_Camera` (`self.PlayerReference`))))))
  (bind _returnvalue (`KismetMathLibrary.MakeRotator` 0.0 _returnvalue_pitch _returnvalue_yaw))
  ;[1 1 1] Spawn Widget Actor
  (bind _returnvalue_2 (`|SpawnActorFromClass` (`self.NPCDialogue_WidgetClassReference`) (`KismetMathLibrary.MakeTransform` (0.0 0.0 0.0) (struct) (0.1 0.1 0.1)) "Undefined" "OverrideRootScale" null null))
  (bind _asbp_npcdialogue_actor_test (cast `/Game/BensTests/DialogueSystemTests/DialogueSystem/BP_NPCDialogueActor_Test` _returnvalue_2))
  (set `self.NPCDialogue_WidgetActorReference` _asbp_npcdialogue_actor_test)
  ;[1 1 1] Rotate/Translate Widget Actor
  (`self.K2_SetActorLocation` (`self.NPCDialogue_WidgetActorReference`) (+ (`SceneComponent.K2_GetComponentLocation` _hmd_camera) (+ (* (`KismetMathLibrary.GetForwardVector` _returnvalue) (`local.ForwardMenuDistance`)) (* (`KismetMathLibrary.GetUpVector` _returnvalue) (`local.UpwardsMenuDistance`)))) false false)
  (`self.K2_SetActorRotation` (`self.NPCDialogue_WidgetActorReference`) (`KismetMathLibrary.MakeRotator` (* _returnvalue_roll -1.0) _returnvalue_pitch_2 _returnvalue_yaw_2) false)
  ;[1 1 1] Attach Widget to Camera
  (`SceneComponent.SetVisibility` (`/Game/BensTests/DialogueSystemTests/DialogueSystem/BP_NPCDialogueActor_Test.NPCDialogue` _npcdialogue_widgetactorreference) true false)
  (`self.K2_AttachToComponent` _npcdialogue_widgetactorreference (`/Game/BensTests/PlayerCharacterTest/NewVRController/MainVRCharacter.HMD_Camera` (`self.PlayerReference`)) "None" "KeepWorld" "KeepWorld" "KeepWorld" false)
  ;[1 1 1] Show Laser Pointers for Player
  (set `WidgetInteractionComponent.bShowDebug` true (`/Game/BensTests/PlayerCharacterTest/NewVRController/MainVRCharacter.L_WidgetInteraction` _playerreference))
  (set `WidgetInteractionComponent.bShowDebug` true (`/Game/BensTests/PlayerCharacterTest/NewVRController/MainVRCharacter.R_WidgetInteraction` _playerreference))
  (set `/Game/BensTests/PlayerCharacterTest/NewVRController/MainVRCharacter.IsMenuActive` true _playerreference))

(fn `UserConstructionScript`)