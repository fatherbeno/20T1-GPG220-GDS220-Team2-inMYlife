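; BP_EnvQGenerator_HightDonut is an EQS generator that produces a donut of query points around the player character.
; It spaces points evenly by angle on concentric rings stepping out from the inner radius, stopping one step short of the outer radius.
; The center is player 0's location projected to navigation, ignoring the supplied context locations.
; All points share a small lift above that center and are not individually projected.
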(fn `DoItemGeneration`
  (params (ContextLocations :type "Array of Vector Structure (by ref)"))
  (bind _points_per_ring (`self.Points Per Ring`))
  (`KismetArrayLibrary.Array_Clear` (`self.Locations`))
  (for _index (range (`self.Number Of Rings`))
    (for _index_2 (range _points_per_ring)
      (`KismetArrayLibrary.Array_Add` (`self.Locations`) (+ (* (`KismetMathLibrary.GreaterGreater_VectorRotator` (1.0 0.0 0.0) (`KismetMathLibrary.MakeRotator` 0.0 0.0 (* _index_2 (/ 360.0 (`KismetMathLibrary.Conv_IntToDouble` _points_per_ring))))) (+ (* (/ (- (`self.Outer Radius`) (`self.Inner Radius`)) (`KismetMathLibrary.Conv_IntToDouble` (`self.Number Of Rings`))) (`KismetMathLibrary.Conv_IntToDouble` _index)) (`self.Inner Radius`))) (`NavigationSystemV1.K2_ProjectPointToNavigation` (`Actor.K2_GetActorLocation` (`GameplayStatics.GetPlayerCharacter` 0))) (0.0 0.0 50.0)))))
  (for _array_element (`self.Locations`)
    (`self.AddGeneratedVector` _array_element))
  (return))