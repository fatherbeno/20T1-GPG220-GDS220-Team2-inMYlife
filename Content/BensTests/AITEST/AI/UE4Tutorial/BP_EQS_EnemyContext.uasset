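; EQS context that supplies the querier's enemy as a single actor for environment queries.
; For AI queriers, it gets the AI controller, casts it to BP_AiController_Runner and returns that controller's Enemy.
; When the querier is an EQSTestingPawn, it returns a ThirdPersonCharacter found in the world instead, so queries work without a controller.
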(fn `ProvideSingleActor`
  (params (QuerierObject :type "Object Object Reference") (QuerierActor :type "Actor Object Reference"))
  (returns (ResultingActor :type "Actor Object Reference"))
  (locals (TempEnemy :type "Actor Object Reference"))
  (bind _returnvalue (`AIBlueprintHelperLibrary.GetAIController` QuerierActor))
  (cast `EQSTestingPawn` QuerierActor
    (:`then`
      (bind _returnvalue_2 (`GameplayStatics.GetActorOfClass` "/Game/ThirdPersonBP/Blueprints/ThirdPersonCharacter.ThirdPersonCharacter_C"))
      (set `local.TempEnemy` _returnvalue_2)
      (return (`local.TempEnemy`)))
    (:`CastFailed`
      (if (!= _returnvalue null)
        (bind _asbp_ai_controller_runner (cast `/Game/BensTests/AITEST/AI/UE4Tutorial/BP_AiController_Runner` _returnvalue))
        (set `local.TempEnemy` (`/Game/BensTests/AITEST/AI/UE4Tutorial/BP_AiController_Runner.Enemy` _asbp_ai_controller_runner))
        (return (`local.TempEnemy`))))))