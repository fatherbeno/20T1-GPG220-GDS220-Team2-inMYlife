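; AI controller for a Runner AI that runs the BT_Runner behavior tree and tracks the player character as its enemy.
; One second after BeginPlay it stores the player in the blackboard as the enemy.
; AI Perception updates involving that enemy refresh a blackboard visibility flag from the success state of the first last-sensed stimulus.
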(event `self.ReceiveBeginPlay`
  (`self.RunBehaviorTree` "/Game/BensTests/AITEST/AI/UE4Tutorial/BT_Runner.BT_Runner")
  (`KismetSystemLibrary.Delay` 1.0)
  (`self.SetEnemy` (`GameplayStatics.GetPlayerCharacter` 0)))

(event `self.AIPerception.OnPerceptionUpdated`
  (params (UpdatedActors :type "Array of Actor Object Reference (by ref)"))
  (for _array_element UpdatedActors
    (if (== _array_element (`self.Enemy`))
      (`self.UpdatePerception` _array_element))))

(fn `SetEnemy`
  (params (NewEnemy :type "Actor Object Reference"))
  (if (!= NewEnemy (`self.Enemy`))
    (bind _output_get (set `self.Enemy` NewEnemy))
    (`BlackboardComponent.SetValueAsObject` (`AIBlueprintHelperLibrary.GetBlackboard` null) "BBK_Enemy" _output_get)
    (`self.UpdatePerception` _output_get)))

(fn `UpdatePerception`
  (params (Enemy :type "Actor Object Reference"))
  (bind _info (`AIPerceptionComponent.GetActorsPerception` (`self.AIPerception`) Enemy))
  (bind (_output_age _output_expirationage _output_strength _output_stimuluslocation _output_receiverlocation _output_tag _output_bsuccessfullysensed) (break `AIStimulus` (`|GetArrayItem` (`.LastSensedStimuli` (break `ActorPerceptionBlueprintInfo` _info)))))
  (`BlackboardComponent.SetValueAsBool` (`AIBlueprintHelperLibrary.GetBlackboard` null) "BBK_IsEnemyVisible" _output_bsuccessfullysensed))

(fn `UserConstructionScript`)