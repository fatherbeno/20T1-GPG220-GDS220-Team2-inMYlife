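; BP_LevelStreamHandler is a test actor that switches streaming sublevel visibility on actor overlap, stepping through a list of load/unload level name pairs.
; Begin overlap sets the current load level's visibility to match whether it is already loaded.
; End overlap hides the current unload level if loaded, then advances the index.
; It never requests loading or unloading, and does not filter overlapping actors.
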(event `self.ReceiveBeginPlay`)

(event `self.ReceiveActorEndOverlap`
  (params (OtherActor :type "Actor Object Reference"))
  (bind (_output_leveltounload _output_leveltoload) (break `/Game/BensTests/LevelStreaming/BPS_LevelStreaming` (`|GetArrayItem` (`self.LevelNames`) (`self.ArrayInt`))))
  (bind _returnvalue (`GameplayStatics.GetStreamingLevel` _output_leveltounload))
  (if (!= "None" _output_leveltounload)
    (if (`LevelStreaming.IsLevelLoaded` _returnvalue)
      (set `LevelStreaming.bShouldBeVisible` false _returnvalue)
      (set `self.ArrayInt` (+ (`self.ArrayInt`) 1)))))

(event `self.ReceiveActorBeginOverlap`
  (params (OtherActor :type "Actor Object Reference"))
  (bind (_output_leveltounload _output_leveltoload) (break `/Game/BensTests/LevelStreaming/BPS_LevelStreaming` (`|GetArrayItem` (`self.LevelNames`) (`self.ArrayInt`))))
  (bind _returnvalue (`GameplayStatics.GetStreamingLevel` _output_leveltoload))
  (if (!= _output_leveltoload "None")
    (set `LevelStreaming.bShouldBeVisible` (`LevelStreaming.IsLevelLoaded` _returnvalue) _returnvalue)))

(fn `UserConstructionScript`)