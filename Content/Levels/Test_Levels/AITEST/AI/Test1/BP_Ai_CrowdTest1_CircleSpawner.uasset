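; Test spawner that places a ring of crowd AI pawns around its capsule for an AI crowd-crossing test.
; On BeginPlay it spawns SpawnCount pawns of the AiSpawning class with BT_CrowdTest1, evenly spaced on a circle of the given Radius.
; Each BP_AICrowdTest1 gets the diametrically opposite point as its TargetLocation.
; The Radius value also offsets the yaw of every spawn angle.
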(event `self.ReceiveBeginPlay`
  (bind _returnvalue (`SceneComponent.K2_GetComponentLocation` (`self.Capsule`)))
  (for _index (range 1 (+ (`self.SpawnCount`) 1))
    (bind _returnvalue_2 (`KismetMathLibrary.GreaterGreater_VectorRotator` (`KismetMathLibrary.MakeVector` (`self.Radius`)) (`KismetMathLibrary.MakeRotator` 0.0 0.0 (+ (`self.Radius`) (* _index (/ 360.0 (`KismetMathLibrary.Conv_IntToDouble` (`self.SpawnCount`))))))))
    (bind _returnvalue_3 (`AIBlueprintHelperLibrary.SpawnAIFromClass` (`self.AiSpawning`) "/Game/Levels/Test_Levels/AITEST/AI/Test1/BT_CrowdTest1.BT_CrowdTest1" (+ _returnvalue _returnvalue_2)))
    (bind _asbp_aicrowd_test_1 (cast `/Game/Levels/Test_Levels/AITEST/AI/Test1/BP_AICrowdTest1` _returnvalue_3))
    (set `/Game/Levels/Test_Levels/AITEST/AI/Test1/BP_AICrowdTest1.TargetLocation` (+ _returnvalue (`KismetMathLibrary.NegateVector` _returnvalue_2)) _asbp_aicrowd_test_1)))

(fn `UserConstructionScript`)